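; Player controller for the hero character that handles movement input and the pause menu.
; Forward and right axis inputs move the pawn along its own facing vectors, but only while the hero is neither attacking nor being attacked.
; Pressing P runs a FlipFlop toggle that swaps the hero's UI with a pause widget created at BeginPlay, switching game pause, input mode and mouse cursor.
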(event Custom|Toggle%20Pause
  (bind _returnvalue (Game|GetPlayerController 0))
  ;[1 1 1] Pause
  (Utilities|FlowControl|FlipFlop
    (:A
      (UserInterface|Viewport|AddtoViewport (Variables|Default|GetPause%20UI) 0)
      (bind _ashero_charater_bp (Utilities|Casting|CastToHeroCharaterBP (Pawn|GetControlledPawn)))
      (Widget|RemovefromParent (Variables|/Game/DFight/Blueprints/Hero/HeroCharaterBP.HeroCharaterBP_C|GetUI _ashero_charater_bp))
      (Input|SetInputModeGameandUI _returnvalue 0 "DoNotLock" true)
      (Variables|/Script/Engine.PlayerController|SetbShowMouseCursor _returnvalue true)
      (Game|SetGamePaused true))
    (:B
      (Widget|RemovefromParent (Variables|Default|GetPause%20UI))
      (bind _ashero_charater_bp_2 (Utilities|Casting|CastToHeroCharaterBP (Pawn|GetControlledPawn)))
      (UserInterface|Viewport|AddtoViewport (Variables|/Game/DFight/Blueprints/Hero/HeroCharaterBP.HeroCharaterBP_C|GetUI _ashero_charater_bp_2) 0)
      (Input|SetInputModeGameOnly _returnvalue)
      (Variables|/Script/Engine.PlayerController|SetbShowMouseCursor _returnvalue false)
      (Game|SetGamePaused false))))

(event EventBeginPlay
  (bind _returnvalue (UserInterface|CreateWidget "/Game/DFight/Blueprints/UI/PauseUI.PauseUI_C"))
  (Variables|Default|SetPause%20UI _returnvalue))

(event EventTick
  (params (DeltaSeconds :type Float%20%28single-precision%29)))

(event Input|AxisEvents|InputAxisMoveForward
  (params (AxisValue :type Float%20%28single-precision%29))
  (bind _returnvalue (Game|Player|GetPlayerPawn 0))
  ;[1 1 1] Movement With WASD
  (Utilities|IsValid _returnvalue
    (:Is%20Valid
      (bind _ashero_charater_bp (Utilities|Casting|CastToHeroCharaterBP _returnvalue))
      (if (not (Variables|/Game/DFight/Blueprints/Hero/HeroCharaterBP.HeroCharaterBP_C|GetIsAttacking _ashero_charater_bp))
        (if (not (Variables|/Game/DFight/Blueprints/Hero/HeroCharaterBP.HeroCharaterBP_C|GetisAttacked _ashero_charater_bp))
          (Pawn|Input|AddMovementInput _returnvalue (Transformation|GetActorForwardVector _returnvalue) AxisValue false))))))

(event Input|AxisEvents|InputAxisMoveRight
  (params (AxisValue :type Float%20%28single-precision%29))
  (bind _returnvalue (Game|Player|GetPlayerPawn 0))
  ;[1 1 1] Movement With WASD
  (Utilities|IsValid _returnvalue
    (:Is%20Valid
      (bind _ashero_charater_bp (Utilities|Casting|CastToHeroCharaterBP _returnvalue))
      (if (not (Variables|/Game/DFight/Blueprints/Hero/HeroCharaterBP.HeroCharaterBP_C|GetIsAttacking _ashero_charater_bp))
        (if (not (Variables|/Game/DFight/Blueprints/Hero/HeroCharaterBP.HeroCharaterBP_C|GetisAttacked _ashero_charater_bp))
          (Pawn|Input|AddMovementInput _returnvalue (Transformation|GetActorRightVector _returnvalue) AxisValue false))))))

(event Input|KeyboardEvents|P
  (params (Key :type Key%20Structure :default "None"))
  ;[1 1 1] Pause
  (:Pressed
    (CallFunction|TogglePause)))

(fn ConstructionScript)