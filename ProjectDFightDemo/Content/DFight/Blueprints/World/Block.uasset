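; Block is a gate-like world actor that switches from a raised, cyan-lit state to a lowered, red-lit state once the hero leaves its trigger box.
; The overlap end clears On and flags Changed, which Tick consumes to call SettingWithOnOff for mesh position, light color and sound.
; The construction script applies the initial state and uses In to choose the trigger's side.
; Nothing here turns On back on.
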(event OnComponentEndOverlap(Box)
  (params (OverlappedComponent :type Primitive%20Component%20Object%20Reference) (OtherActor :type Actor%20Object%20Reference) (OtherComp :type Primitive%20Component%20Object%20Reference) (OtherBodyIndex :type Integer))
  (Utilities|Casting|CastToHeroCharaterBP OtherActor)
  (if (Variables|Default|Geton)
    (Variables|Default|Seton false)
    (Variables|Default|Setchanged true)))

(event EventBeginPlay)

(event Collision|EventActorBeginOverlap
  (params (OtherActor :type Actor%20Object%20Reference)))

(event EventTick
  (params (DeltaSeconds :type Float%20%28single-precision%29))
  (if (Variables|Default|Getchanged)
    (CallFunction|SettingwithonOff)
    (Variables|Default|Setchanged false)))

(fn ConstructionScript
  (bind _box (Variables|Default|GetBox))
  (Utilities|FlowControl|Sequence
    (:then_0
      (CallFunction|SettingwithonOff))
    (:then_1
      (if (Variables|Default|Getin)
        (Transformation|SetRelativeLocation _box "-200.000000,0.000000,125.000000" false false)
        (else
          (Transformation|SetRelativeLocation _box "200.000000,0.000000,125.000000" false false))))))

(fn SettingwithonOff
  (if (Variables|Default|Geton)
    (Rendering|Components|Light|SetLightColor (Variables|Default|GetPointLight) "(R=0.000000,G=0.893492,B=1.000000,A=1.000000)" true)
    (Transformation|SetRelativeLocation (Variables|Default|GetStaticMesh) "0, 0,315.000000" false false)
    (Audio|PlaySoundatLocation "/Engine/VREditor/Sounds/UI/Dockable_Window_Drop.Dockable_Window_Drop" (Transformation|GetActorLocation) "0, 0, 0" 1.0 1.0 0.0 0 0 0)
    (else
      (Rendering|Components|Light|SetLightColor (Variables|Default|GetPointLight) "(R=1.000000,G=0.191202,B=0.000000,A=1.000000)" true)
      (Transformation|SetRelativeLocation (Variables|Default|GetStaticMesh) "0, 0,65.000000" false false)
      (Transformation|SetRelativeLocation (Variables|Default|GetStaticMesh1) "0, 0,100.000000" false false)
      (Audio|PlaySoundatLocation "/Engine/VREditor/Sounds/UI/Dockable_Window_Close.Dockable_Window_Close" (Transformation|GetActorLocation) "0, 0, 0" 1.0 1.0 0.0 0 0 0))))