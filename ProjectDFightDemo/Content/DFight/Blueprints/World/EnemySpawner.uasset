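; A one-shot proximity spawner that releases a group of spider monsters when the player comes close.
; Tick checks the distance to the player pawn until it falls within range, then sets a flag, turns the point light orange and plays a sound.
; A loop spawns the spiders at random navigable points around the spawner at a fixed height, each playing a teleport animation.
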(event EventBeginPlay)

(event Collision|EventActorBeginOverlap
  (params (OtherActor :type Actor%20Object%20Reference)))

(event EventTick
  (params (DeltaSeconds :type Float%20%28single-precision%29))
  (bind _returnvalue (Transformation|GetActorLocation))
  (if (not (Variables|Default|GetSpawned))
    (if (< (Math|Vector|VectorLength (- _returnvalue (Transformation|GetActorLocation (Game|Player|GetPlayerPawn 0)))) 5e+02)
      (Variables|Default|SetSpawned true)
      (Rendering|Components|Light|SetLightColor (Variables|Default|GetPointLight) "(R=1.000000,G=0.500000,B=0.000000,A=1.000000)" true)
      (Audio|PlaySoundatLocation "/Engine/EditorSounds/Notifications/CompileFailed.CompileFailed" _returnvalue "0, 0, 0" 1.0 1.0 0.0 0 0 0)
      (for _index (range 0 5)
        (bind _randomlocation (Class|NavigationSystemV1|GetRandomLocationinNavigableRadius _returnvalue 1e+03 0 0))
        (bind _returnvalue_2 (Game|SpawnActorfromClass "/Game/DFight/Blueprints/Spider/SpiderMonsterBP.SpiderMonsterBP_C" (Math|Transform|MakeTransform (Math|Vector|MakeVector (.X (Math|Vector|BreakVector _randomlocation)) (.Y (Math|Vector|BreakVector _randomlocation)) 6e+02)) "Undefined" 0 0))
        (Components|Animation|PlayAnimation (Variables|/Script/Engine.Character|GetMesh _returnvalue_2) "/Game/InfinityBladeAdversaries/Enemy/Enemy_Great_Spider/Enemy_SpiderGreater_Animation/ExoGame_Greater_Spider_Teleport.ExoGame_Greater_Spider_Teleport" false)))))

(fn ConstructionScript)