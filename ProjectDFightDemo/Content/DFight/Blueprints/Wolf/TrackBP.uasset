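; TrackBP is a track actor that lays out a circular spline path of a given Radius around its origin.
; The construction script clears the spline and rebuilds it from points placed by sine and cosine on the local XY plane.
; The point count scales with Radius, so spacing stays roughly constant as the circle grows.
; The event graph holds only disabled placeholder events, so the actor has no runtime logic.
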(event EventBeginPlay)

(event Collision|EventActorBeginOverlap
  (params (OtherActor :type Actor%20Object%20Reference)))

(event EventTick
  (params (DeltaSeconds :type Float%20%28single-precision%29)))

(fn ConstructionScript
  (bind _radius (Variables|Default|GetRadius))
  (Spline|ClearSplinePoints (Variables|Default|GetSpline) true)
  (bind _output_get (Variables|Default|SetPoints%20Count (Math|Float|Round (/ (Variables|Default|GetRadius) 2e+02))))
  (for _index (range 0 _output_get)
    (Class|SplineComponent|AddPoint (Variables|Default|GetSpline) (Utilities|Struct|MakeSplinePoint (Math|Conversions|ToFloat(Integer) _index) (Math|Vector|MakeVector (* (Math|Trig|Cos(Degrees) (* _index (/ 3.6e+02 (Math|Conversions|ToFloat(Integer) _output_get)))) _radius) (* (Math|Trig|Sin(Degrees) (* _index (/ 3.6e+02 (Math|Conversions|ToFloat(Integer) _output_get)))) _radius) 0.0)) true)))