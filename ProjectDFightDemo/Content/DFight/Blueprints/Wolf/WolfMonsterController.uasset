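; AI controller for the wolf monster that runs the WolfMonsterBT behavior tree when it possesses a WolfMonsterBP.
; Every tick it sets the blackboard TargetActor to player pawn 0 when within a fixed radius, and clears it otherwise.
; An AI Perception update checks for a sensed "Hero"-tagged actor, but both branches write an empty TargetActor, so only the distance check supplies a target.
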(event OnTargetPerceptionUpdated(AIPerception)
  (params (Actor :type Actor%20Object%20Reference) (Stimulus :type AI%20Stimulus%20Structure))
  (bind _returnvalue (Utilities|Name|MakeLiteralName "TargetActor"))
  (bind _blackboard (Variables|Default|GetBlackboard))
  (if (and (Actor|ActorHasTag Actor "Hero") (.bSuccessfullySensed (Utilities|Struct|BreakAIStimulus Stimulus)))
    (AI|Components|Blackboard|SetValueasObject _blackboard _returnvalue 0)
    (else
      (AI|Components|Blackboard|SetValueasObject _blackboard _returnvalue 0))))

(event EventBeginPlay)

(event EventTick
  (params (DeltaSeconds :type Float%20%28single-precision%29))
  (bind _returnvalue (Game|Player|GetPlayerPawn 0))
  (bind _returnvalue_2 (Utilities|Name|MakeLiteralName "TargetActor"))
  (bind _blackboard (Variables|Default|GetBlackboard))
  ;[1 1 1] Find Hero
  (if (< (Math|Vector|VectorLength (- (Transformation|GetActorLocation _returnvalue) (Transformation|GetActorLocation (Pawn|GetControlledPawn)))) 1e+03)
    (AI|Components|Blackboard|SetValueasObject _blackboard _returnvalue_2 _returnvalue)
    (else
      (AI|Components|Blackboard|SetValueasObject _blackboard _returnvalue_2 0))))

(event EventPossess
  (params (PossessedPawn :type Pawn%20Object%20Reference))
  (Utilities|Casting|CastToWolfMonsterBP PossessedPawn)
  (AI|RunBehaviorTree "/Game/DFight/Blueprints/Wolf/BT/WolfMonsterBT.WolfMonsterBT"))

(fn ConstructionScript)