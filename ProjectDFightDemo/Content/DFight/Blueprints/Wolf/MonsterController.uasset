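; MonsterController is the AI controller that makes a WolfBP patrol along a spline track.
; On BeginPlay it casts the controlled pawn to WolfBP and caches the spline from its PatrolTrack along with the point count.
; MoveToPoint increments the wolf's CurrentPoint with wraparound, sends it there with AIMoveTo, and calls itself on success for an endless loop.
; A failed move has no handler, so the patrol does not continue.
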(event Custom|Move%20to%20Point
  (bind _output_get (Variables|/Game/DFight/Blueprints/Wolf/WolfBP.WolfBP_C|SetCurrentPoint (stale EventBeginPlay _aswolf_bp) (Math|Integer|%(Integer) (+ (Variables|/Game/DFight/Blueprints/Wolf/WolfBP.WolfBP_C|GetCurrentPoint (stale EventBeginPlay _aswolf_bp)) 1) (Variables|Default|GetNum%20of%20Points))))
  (AI|AIMoveTo (Pawn|GetControlledPawn) (Spline|GetLocationatSplinePoint (Variables|Default|GetSpline) _output_get "World") 0 1e+01 false
    (:OnSuccess
      (CallFunction|MovetoPoint))))

(event EventBeginPlay
  (bind _aswolf_bp (Utilities|Casting|CastToWolfBP (Pawn|GetControlledPawn)))
  (bind _output_get (Variables|Default|SetSpline (Variables|/Game/DFight/Blueprints/Wolf/TrackBP.TrackBP_C|GetSpline (Variables|/Game/DFight/Blueprints/Wolf/WolfBP.WolfBP_C|GetPatrol%20Track _aswolf_bp))))
  (Variables|Default|SetNum%20of%20Points (Spline|GetNumberOfSplinePoints _output_get))
  (CallFunction|MovetoPoint))

(fn ConstructionScript)