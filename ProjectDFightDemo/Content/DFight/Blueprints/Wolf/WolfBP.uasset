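; WolfBP is a damageable wolf actor that reacts to hits and dies when its HP runs out.
; AnyDamage subtracts truncated damage from HP, plays a front-hit animation directly on the skeletal mesh and plays a quiet sound at the wolf's location.
; At zero or lower HP, a death animation replaces the hit reaction, collision turns off and the actor is destroyed after a short delay.
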(event EventBeginPlay)

(event Collision|EventActorBeginOverlap
  (params (OtherActor :type Actor%20Object%20Reference)))

(event EventTick
  (params (DeltaSeconds :type Float%20%28single-precision%29)))

(event Game|Damage|EventAnyDamage
  (params (Damage :type Float%20%28single-precision%29) (DamageType :type Damage%20Type%20Object%20Reference) (InstigatedBy :type Controller%20Object%20Reference) (DamageCauser :type Actor%20Object%20Reference))
  (bind _output_get (Variables|Default|SetHP (- (Variables|Default|GetHP) (Math|Float|Truncate Damage))))
  (Components|Animation|PlayAnimation (Variables|Default|GetSkeletalMesh) "/Game/AnimalVarietyPack/Wolf/Animations/ANIM_Wolf_GetHitFront.ANIM_Wolf_GetHitFront" false)
  (Audio|PlaySoundatLocation "/Engine/EditorSounds/GamePreview/EjectFromPlayer.EjectFromPlayer" (Transformation|GetActorLocation) "0, 0, 0" 0.25 1.0 0.0 0 0 0)
  (if (<= _output_get 0)
    (Components|Animation|PlayAnimation (Variables|Default|GetSkeletalMesh) "/Game/AnimalVarietyPack/Wolf/Animations/ANIM_Wolf_Death.ANIM_Wolf_Death" false)
    (Collision|SetActorEnableCollision false)
    (Utilities|FlowControl|Delay 3.0)
    (Actor|DestroyActor)))

(fn ConstructionScript)