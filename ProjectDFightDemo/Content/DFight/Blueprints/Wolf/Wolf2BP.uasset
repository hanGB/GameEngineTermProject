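; Wolf enemy actor that takes damage, shows an on-screen UI and dies when its HP runs out.
; Each tick it projects the widget above its head while the player is within range, hiding it otherwise.
; Damage updates the HP bar and plays a hit animation and sound; Tick restores the anim class once playback stops.
; At zero HP it plays death, disables collision, removes the UI and destroys itself after a delay.
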(event EventBeginPlay
  (bind _returnvalue (UserInterface|CreateWidget "/Game/DFight/Blueprints/Wolf/Monster2UI.Monster2UI_C" 0 self))
  (Variables|Default|SetUI _returnvalue)
  (Variables|Default|SetHP (Variables|Default|GetMaxHP))
  (Variables|Default|SetPlayer (Game|Player|GetPlayerPawn 0))
  (UserInterface|Viewport|AddtoViewport (Variables|Default|GetUI) 0))

(event EventTick
  (params (DeltaSeconds :type Float%20%28single-precision%29))
  (Utilities|FlowControl|Sequence
    (:then_0
      (if (< (Math|Vector|VectorLength (- (Transformation|GetActorLocation (Variables|Default|GetPlayer)) (Transformation|GetActorLocation))) (Variables|Default|Getui%20seen%20distance))
        (CallFunction|UpdaetUIPosition)
        (Widget|SetVisibility (Variables|Default|GetUI) "Visible")
        (else
          (Widget|SetVisibility (Variables|Default|GetUI) "Hidden"))))
    (:then_1
      (if (not (Audio|Components|Audio|IsPlaying (Variables|Character|GetMesh)))
        (Class|SkeletalMeshComponent|SetAnimClass (Variables|Character|GetMesh) "/Game/DFight/Blueprints/Wolf/WolfAnimation.WolfAnimation_C")))))

(event Game|Damage|EventAnyDamage
  (params (Damage :type Float%20%28single-precision%29) (DamageType :type Damage%20Type%20Object%20Reference) (InstigatedBy :type Controller%20Object%20Reference) (DamageCauser :type Actor%20Object%20Reference))
  (bind _output_get (Variables|Default|SetHP (- (Variables|Default|GetHP) (Math|Float|Truncate Damage))))
  (Default|CallUpdateHPBarUI)
  (Components|Animation|PlayAnimation (Variables|Character|GetMesh) "/Game/AnimalVarietyPack/Wolf/Animations/ANIM_Wolf_GetHitFront.ANIM_Wolf_GetHitFront" false)
  (Audio|PlaySoundatLocation "/Engine/EditorSounds/GamePreview/EjectFromPlayer.EjectFromPlayer" (Transformation|GetActorLocation) "0, 0, 0" 0.25 1.0 0.0 0 0 0)
  (if (<= _output_get 0)
    (Components|Animation|PlayAnimation (Variables|Character|GetMesh) "/Game/AnimalVarietyPack/Wolf/Animations/ANIM_Wolf_Death.ANIM_Wolf_Death" false)
    (Collision|SetActorEnableCollision false)
    (Widget|RemovefromParent (Variables|Default|GetUI))
    (Utilities|FlowControl|Delay 2.0)
    (Actor|DestroyActor)))

(fn ConstructionScript)

(fn UpdaetUIPosition
  (Class|UserWidget|SetPositioninViewport (Variables|Default|GetUI) (.ScreenLocation (Class|PlayerController|ProjectWorldLocationtoScreen (Game|GetPlayerController 0) (+ (Transformation|GetActorLocation) "0, 0,125.000000") false)) true))