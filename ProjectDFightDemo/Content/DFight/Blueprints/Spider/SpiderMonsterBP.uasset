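; Spider enemy Blueprint that fights the hero, with its own health bar widget and left and right damage boxes that hurt the hero on overlap.
; Tick projects the bar above the spider while the player is near and restores the animation Blueprint after one-shot animations end.
; Taking damage plays a reaction and screech, then teleports it back from the player after a delay.
; At zero HP it plays death, fires a dead dispatcher and destroys itself.
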(event OnComponentBeginOverlap(LeftDamageBox)
  (params (OverlappedComponent :type Primitive%20Component%20Object%20Reference) (OtherActor :type Actor%20Object%20Reference) (OtherComp :type Primitive%20Component%20Object%20Reference) (OtherBodyIndex :type Integer) (bFromSweep :type Boolean) (SweepResult :type Hit%20Result%20Structure%20%28by%20ref%29))
  ;[1 1 1] Apply damage to hero
  (bind _ashero_charater_bp (Utilities|Casting|CastToHeroCharaterBP OtherActor))
  (Game|Damage|ApplyDamage _ashero_charater_bp 8.0 0 0)
  (Variables|/Script/Engine.PrimitiveComponent|SetbGenerateOverlapEvents (Variables|Default|GetLeftDamageBox) false))

(event OnComponentBeginOverlap(RightDamageBox)
  (params (OverlappedComponent :type Primitive%20Component%20Object%20Reference) (OtherActor :type Actor%20Object%20Reference) (OtherComp :type Primitive%20Component%20Object%20Reference) (OtherBodyIndex :type Integer) (bFromSweep :type Boolean) (SweepResult :type Hit%20Result%20Structure%20%28by%20ref%29))
  ;[1 1 1] Apply damage to hero
  (bind _ashero_charater_bp (Utilities|Casting|CastToHeroCharaterBP OtherActor))
  (Game|Damage|ApplyDamage _ashero_charater_bp 8.0 0 0)
  (Variables|/Script/Engine.PrimitiveComponent|SetbGenerateOverlapEvents (Variables|Default|GetRightDamageBox) false))

(event EventBeginPlay
  ;[1 1 1] Create hp bar ui
  (bind _returnvalue (UserInterface|CreateWidget "/Game/DFight/Blueprints/Spider/SpiderMonsterUI.SpiderMonsterUI_C" 0 self))
  (Variables|Default|SetUI _returnvalue)
  (Variables|Default|SetHP (Variables|Default|GetMaxHP))
  (Variables|Default|SetPlayer (Game|Player|GetPlayerPawn 0))
  (UserInterface|Viewport|AddtoViewport (Variables|Default|GetUI) 0))

(event EventTick
  (params (DeltaSeconds :type Float%20%28single-precision%29))
  ;[1 1 1] Animation and ui update
  (Utilities|FlowControl|Sequence
    (:then_0
      (if (< (Math|Vector|VectorLength (- (Transformation|GetActorLocation (Variables|Default|GetPlayer)) (Transformation|GetActorLocation))) (Variables|Default|Getui%20seen%20distance))
        (CallFunction|UpdaetUIPosition)
        (Widget|SetVisibility (Variables|Default|GetUI) "Visible")
        (else
          (Widget|SetVisibility (Variables|Default|GetUI) "Hidden"))))
    (:then_1
      (if (not (Audio|Components|Audio|IsPlaying (Variables|Character|GetMesh)))
        (if (not (Variables|Default|GetisDead))
          (Class|SkeletalMeshComponent|SetAnimClass (Variables|Character|GetMesh) "/Game/DFight/Blueprints/Spider/SpiderMonsterAnimationBP.SpiderMonsterAnimationBP_C")
          (Variables|Default|SetisAttacked false))))))

(event Game|Damage|EventAnyDamage
  (params (Damage :type Float%20%28single-precision%29) (DamageType :type Damage%20Type%20Object%20Reference) (InstigatedBy :type Controller%20Object%20Reference) (DamageCauser :type Actor%20Object%20Reference))
  ;[1 1 1] Apply Damage
  (Variables|Default|SetisAttacked true)
  (bind _output_get (Variables|Default|SetHP (- (Variables|Default|GetHP) (Math|Float|Truncate Damage))))
  (Default|CallUpdateHPBarUISpider)
  (Components|Animation|PlayAnimation (Variables|Character|GetMesh) "/Game/InfinityBladeAdversaries/Enemy/Enemy_Great_Spider/Enemy_SpiderGreater_Animation/ExoGame_Greater_Spider_React_Heavy_Front.ExoGame_Greater_Spider_React_Heavy_Front" false)
  (Audio|PlaySoundatLocation "/Game/FarmAnimalSounds/Animals/Horse/cue/Horse_Screech_03_Cue.Horse_Screech_03_Cue" (Transformation|GetActorLocation) "0, 0, 0" 1.0 1.0 0.0 0 0 0)
  (if (<= _output_get 0)
    (Components|Animation|PlayAnimation (Variables|Character|GetMesh) "/Game/InfinityBladeAdversaries/Enemy/Enemy_Great_Spider/Enemy_SpiderGreater_Animation/ExoGame_Greater_Spider_Death.ExoGame_Greater_Spider_Death" false)
    (Collision|SetActorEnableCollision false)
    (Widget|RemovefromParent (Variables|Default|GetUI))
    (Variables|Default|SetisDead true)
    (Utilities|FlowControl|Delay 2.0)
    (Default|CallSpiderDead)
    (Actor|DestroyActor)
    (else
      (Utilities|FlowControl|Delay 1.18)
      (Transformation|AddActorWorldOffset (* (Math|Vector|Normalize (- (Transformation|GetActorLocation) (Transformation|GetActorLocation (Game|Player|GetPlayerPawn 0)))) 8e+01) false true))))

(fn ConstructionScript)

(fn UpdaetUIPosition
  (Class|UserWidget|SetPositioninViewport (Variables|Default|GetUI) (.ScreenLocation (Class|PlayerController|ProjectWorldLocationtoScreen (Game|GetPlayerController 0) (+ (Transformation|GetActorLocation) "0, 0,125.000000") false)) true))