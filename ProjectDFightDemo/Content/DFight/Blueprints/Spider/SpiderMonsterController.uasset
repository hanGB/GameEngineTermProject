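; AI controller for the spider monster that runs its behavior tree and feeds it patrol and target data through the Blackboard.
; On possess, track-bound spiders read their patrol spline, and SetNextPoint cycles through its points into TargetPoint.
; Tick detects the player by distance, setting or clearing TargetActor and yawing a nearby spider toward them unless dead or attacked.
; The AI Perception handler only writes an empty TargetActor on both branches.
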(event OnTargetPerceptionUpdated(AIPerception)
  (params (Actor :type Actor%20Object%20Reference) (Stimulus :type AI%20Stimulus%20Structure))
  (bind _returnvalue (Utilities|Name|MakeLiteralName "TargetActor"))
  (bind _blackboard (Variables|Default|GetBlackboard))
  (if (and (Actor|ActorHasTag Actor "Hero") (.bSuccessfullySensed (Utilities|Struct|BreakAIStimulus Stimulus)))
    (AI|Components|Blackboard|SetValueasObject _blackboard _returnvalue 0)
    (else
      (AI|Components|Blackboard|SetValueasObject _blackboard _returnvalue 0))))

(event Custom|SetNextPoint
  (bind _asspider_monster_bp (Utilities|Casting|CastToSpiderMonsterBP (Pawn|GetControlledPawn)))
  (bind _output_get (Variables|/Game/DFight/Blueprints/Spider/SpiderMonsterBP.SpiderMonsterBP_C|SetCurrentPoint _asspider_monster_bp (Math|Integer|%(Integer) (+ (Variables|/Game/DFight/Blueprints/Spider/SpiderMonsterBP.SpiderMonsterBP_C|GetCurrentPoint _asspider_monster_bp) 1) (Variables|Default|GetNumOfSplinePoints))))
  (AI|Components|Blackboard|SetValueasVector (AI|GetBlackboard self) (Utilities|Name|MakeLiteralName "TargetPoint") (Spline|GetLocationatSplinePoint (Variables|Default|GetSpline) _output_get "World")))

(event EventBeginPlay)

(event EventTick
  (params (DeltaSeconds :type Float%20%28single-precision%29))
  (bind _returnvalue (Game|Player|GetPlayerPawn 0))
  (bind _returnvalue_2 (Utilities|Name|MakeLiteralName "TargetActor"))
  (bind _returnvalue_3 (Pawn|GetControlledPawn))
  (bind _blackboard (Variables|Default|GetBlackboard))
  (bind _returnvalue_4 (Transformation|GetActorLocation _returnvalue_3))
  (bind _returnvalue_5 (Transformation|GetActorLocation _returnvalue))
  (bind _returnvalue_6 (- _returnvalue_5 _returnvalue_4))
  (bind (_x _y) (Math|Vector|BreakVector _returnvalue_6))
  ;[1 1 1] Find Hero
  (if (< (Math|Vector|VectorLength _returnvalue_6) 1e+03)
    (AI|Components|Blackboard|SetValueasObject _blackboard _returnvalue_2 _returnvalue)
    (bind _asspider_monster_bp (Utilities|Casting|CastToSpiderMonsterBP _returnvalue_3))
    (if (not (or (Variables|/Game/DFight/Blueprints/Spider/SpiderMonsterBP.SpiderMonsterBP_C|GetisDead _asspider_monster_bp) (Variables|/Game/DFight/Blueprints/Spider/SpiderMonsterBP.SpiderMonsterBP_C|GetisAttacked _asspider_monster_bp)))
      (Transformation|SetActorRotation _returnvalue_3 (Math|Rotator|MakeRotator 0.0 0.0 (Class|KismetMathLibrary|DegAtan2 _y _x))))
    (else
      (AI|Components|Blackboard|SetValueasObject _blackboard _returnvalue_2 0))))

(event EventPossess
  (params (PossessedPawn :type Pawn%20Object%20Reference))
  (bind _asspider_monster_bp (Utilities|Casting|CastToSpiderMonsterBP PossessedPawn))
  (AI|RunBehaviorTree "/Game/DFight/Blueprints/Spider/BT/SpiderMonsterBT.SpiderMonsterBT")
  (if (Variables|/Game/DFight/Blueprints/Spider/SpiderMonsterBP.SpiderMonsterBP_C|GetisInTrack _asspider_monster_bp)
    (bind _output_get (Variables|Default|SetSpline (Variables|/Game/DFight/Blueprints/Wolf/TrackBP.TrackBP_C|GetSpline (Variables|/Game/DFight/Blueprints/Spider/SpiderMonsterBP.SpiderMonsterBP_C|GetPatrol%20Track _asspider_monster_bp))))
    (Variables|Default|SetNumOfSplinePoints (Spline|GetNumberOfSplinePoints _output_get))
    (CallFunction|SetNextPoint)))

(fn ConstructionScript)